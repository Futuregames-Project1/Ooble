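; Player controller for the submarine that swaps HUD widgets, aims the flashlight and tracks energy.
; It shows the pearl counter at start, then replaces all widgets for game over, victory or menu screens, with debug inputs for instant win and FPS stats.
; Tick rotates the submarine's spotlight toward the right stick or cursor trace, storing the aim rotation.
; Tick also updates energy, killing the player at zero, otherwise updating projectile delay.
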(event Custom|CrashScreen
  ;[1 1 1] Add Game Over HUD to the view
  (Utilities|FlowControl|Delay 1.0)
  (Viewport|RemoveAllWidgets)
  (bind _returnvalue (UserInterface|CreateWidget "/Game/Assets/Blueprints/Widgets/GameOverScreen_HUD.GameOverScreen_HUD_C"))
  (UserInterface|Viewport|AddtoViewport _returnvalue 0))

(event Custom|WinScreen
  ;[1 1 1] Add Victory Screen HUD to the view
  (Viewport|RemoveAllWidgets)
  (bind _returnvalue (UserInterface|CreateWidget "/Game/Assets/Blueprints/Widgets/VictoryScreen_HUD.VictoryScreen_HUD_C"))
  (UserInterface|Viewport|AddtoViewport _returnvalue 0))

(event Custom|MenuScreen
  ;[1 1 1] Add Menu HUD to the View
  (Viewport|RemoveAllWidgets)
  (bind _returnvalue (UserInterface|CreateWidget "/Game/Assets/Blueprints/Widgets/MenuScreen_HUD.MenuScreen_HUD_C"))
  (UserInterface|Viewport|AddtoViewport _returnvalue 0))

(event EventTick
  (params (DeltaSeconds :type Float%20%28single-precision%29))
  (Utilities|FlowControl|Sequence
    (:then_0
      (if (Variables|Default|GetbRotateFlashligt?)
        (bind _assubmarine_bp (Utilities|Casting|CastToSubmarine_BP (Pawn|GetControlledPawn)))
        (if (Variables|Default|GetUseController)
          (Transformation|SetWorldRotation (Variables|/Game/Assets/Blueprints/Submarine_BP.Submarine_BP_C|GetSpotLight _assubmarine_bp) (Math|Rotator|FindLookatRotation (Transformation|GetWorldLocation (Variables|/Game/Assets/Blueprints/Submarine_BP.Submarine_BP_C|GetSpotLight _assubmarine_bp)) (+ (Variables|Default|GetRightStickRotation) (Transformation|GetWorldLocation (Variables|/Game/Assets/Blueprints/Submarine_BP.Submarine_BP_C|GetSpotLight _assubmarine_bp)))) false false)
          (Variables|Default|SetAimRotation (Math|Rotator|FindLookatRotation (Transformation|GetWorldLocation (Variables|/Game/Assets/Blueprints/Submarine_BP.Submarine_BP_C|GetSpotLight _assubmarine_bp)) (+ (Variables|Default|GetRightStickRotation) (Transformation|GetWorldLocation (Variables|/Game/Assets/Blueprints/Submarine_BP.Submarine_BP_C|GetSpotLight _assubmarine_bp)))))
          (else
            (Transformation|SetWorldRotation (Variables|/Game/Assets/Blueprints/Submarine_BP.Submarine_BP_C|GetSpotLight _assubmarine_bp) (Math|Rotator|MakeRotator 0.0 0.0 (.Yaw (Math|Rotator|BreakRotator (Math|Rotator|FindLookatRotation (Transformation|GetWorldLocation (Variables|/Game/Assets/Blueprints/Submarine_BP.Submarine_BP_C|GetSpotLight _assubmarine_bp)) (.Location (Collision|BreakHitResult (.HitResult (Game|Player|GetHitResultUnderCursorbyChannel "TraceTypeQuery3" true)))))))) false false)
            (Variables|Default|SetAimRotation (Math|Rotator|MakeRotator 0.0 0.0 (.Yaw (Math|Rotator|BreakRotator (Math|Rotator|FindLookatRotation (Transformation|GetWorldLocation (Variables|/Game/Assets/Blueprints/Submarine_BP.Submarine_BP_C|GetSpotLight _assubmarine_bp)) (.Location (Collision|BreakHitResult (.HitResult (Game|Player|GetHitResultUnderCursorbyChannel "TraceTypeQuery3" true)))))))))))))
    (:then_1
      ;[1 1 1] Calculate Current Energy
      (bind _output_get (Variables|Default|SetCurrentEnergy (Utilities|CalculateCurrentEnergy)))
      ;[1 1 1] Check if energy is Zero
      (if (<= _output_get 0.0)
        ;[1 1 1] Player Death
        (bind _assubmarine_bp_2 (Utilities|Casting|CastToSubmarine_BP (Game|Player|GetPlayerPawn 0)))
        (Default|PlayerDeath _assubmarine_bp_2)
        (else
          ;[1 1 1] Calculate Current Projectile Delay
          (Variables|Default|SetCurrentProjectileDelay (Utilities|CalculateCurrentProjectileDelay)))))))

(event EventBeginPlay
  ;[1 1 1] Add Pearlcounter HUD to the view
  (bind _returnvalue (UserInterface|CreateWidget "/Game/Assets/Blueprints/Widgets/PearlCounter_HUD.PearlCounter_HUD_C"))
  (UserInterface|Viewport|AddtoViewport _returnvalue 0))

(event Input|ActionEvents|InputActionFPS
  (params (Key :type Key%20Structure :default "AnyKey"))
  (:Pressed
    (Development|ExecuteConsoleCommand "stat FPS")))

(event Input|ActionEvents|InputActionWin
  (params (Key :type Key%20Structure :default "AnyKey"))
  (:Pressed
    (Development|PrintString "Cheater")
    ;[1 1 1] Add Victory Screen HUD to the view
    (Viewport|RemoveAllWidgets)
    (bind _returnvalue (UserInterface|CreateWidget "/Game/Assets/Blueprints/Widgets/VictoryScreen_HUD.VictoryScreen_HUD_C"))
    (UserInterface|Viewport|AddtoViewport _returnvalue 0)))

(fn ConstructionScript)