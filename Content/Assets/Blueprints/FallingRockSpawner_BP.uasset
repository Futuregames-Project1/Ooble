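; Actor Blueprint that periodically spawns FallingRock_BP actors at its own location as a timed rockfall hazard.
; After a random initial delay on BeginPlay, a looping Delay chain spawns enlarged rocks at the root component's location and rotation, with random intervals between spawns.
; A parallel sequence branch destroys the spawner after a fixed lifetime, counted from the first spawn, which ends the loop.
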(event EventBeginPlay
  (bind _self self)
  (bind _initialrockspawningdelay (Variables|Default|GetInitialRockSpawningDelay))
  (bind _rockspawningdelay (Variables|Default|GetRockSpawningDelay))
  (bind _defaultsceneroot (Variables|Default|GetDefaultSceneRoot _self))
  (Utilities|FlowControl|Delay (Math|Random|RandomFloatinRange (.x _initialrockspawningdelay) (.y _initialrockspawningdelay)))
  (Utilities|FlowControl|Sequence
    (:then_0
      (Game|SpawnActorfromClass "/Game/Assets/Blueprints/FallingRock_BP.FallingRock_BP_C" (Math|Transform|MakeTransform (Transformation|GetWorldLocation _defaultsceneroot) (Transformation|GetWorldRotation _defaultsceneroot) "25.000000,25.000000,25.000000") "Undefined" 0 0 :!label _label)
      (Utilities|FlowControl|Delay (Math|Random|RandomFloatinRange (.x _rockspawningdelay) (.y _rockspawningdelay)))
      (goto _label))
    (:then_1
      (Utilities|FlowControl|Delay 3e+01)
      (Actor|DestroyActor))))

(fn ConstructionScript)