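; Destructible rock actor that breaks apart when its Destroy event is called and signals the player's submarine to move its camera.
; Destroy shrinks the actor, applies damage to the Destructible component, plays a crack sound and disables collision on RockMesh.
; It then sets MoveCamera on the player's Submarine_BP pawn and removes the actor after a delay, provided that cast succeeds.
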(event Custom|Destroy
  (bind _destructible (Variables|Default|GetDestructible))
  (bind _returnvalue (Transformation|GetWorldLocation _destructible))
  (Transformation|SetActorScale3D (* (Transformation|GetActorScale3D self) 0.25))
  (Game|Damage|ApplyDamage _destructible 1.0 _returnvalue _returnvalue 0.0)
  (Audio|PlaySoundatLocation "/Game/Assets/Sounds/RocksCrack.RocksCrack" _returnvalue)
  (Collision|SetCollisionEnabled (Variables|Default|GetRock_Mesh) "NoCollision")
  (bind _assubmarine_bp (Utilities|Casting|CastToSubmarine_BP (Game|Player|GetPlayerPawn 0)))
  (Variables|/Game/Assets/Blueprints/Submarine_BP.Submarine_BP_C|SetMoveCamera _assubmarine_bp true)
  (Utilities|FlowControl|Delay 1e+01)
  (Actor|DestroyActor))

(fn ConstructionScript)