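; Player submarine for an auto-scrolling underwater game, with shooting, pickups and energy-based damage.
; Tick carries the actor and camera along a spline while moving the Player component within it using input velocity, friction and fake gravity.
; Overlaps dispatch by actor tag to obstacles, pickups or the win screen, with damage granting red-flashing invincibility.
; Submarine_Con holds aim, energy, fire cooldown and screens; debug inputs control camera speed and damage immunity.
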(event Custom|Invincibility
  ;[0.735 0.08452 0.08452] Playe Invincibility
  (Variables|Default|SetPlayerInvincible true)
  (Effects|SpawnEmitteratLocation "/Game/Assets/Particles/BubbleExplosionv2.BubbleExplosionv2" (Transformation|GetWorldLocation (Variables|Default|GetSubmarine_mesh)))
  ;[1 1 1] Makes player flash red
  (Utilities|InvincibleTimer (Variables|Default|GetInvincibilityTime)
    (:Output
      (if (Variables|Default|GetPlayerInvincible) :!label _label
        (Utilities|FlashMaterial
          (:Output
            (goto _label)))))
    (:TimerDone
      (Variables|Default|SetPlayerInvincible false))))

(event Custom|CameraShake
  (params (Shake :type Camera%20Shake%20Class%20Reference))
  ;[1 1 1] Camera Shake
  (Camera|PlayWorldCameraShake Shake (Transformation|GetActorLocation self) 0.0 5.0))

(event EventTick
  (params (DeltaSeconds :type Float%20%28single-precision%29))
  (bind _submarinemovement (Variables|Default|GetSubmarineMovement))
  ;[0.735 0.08452 0.08452] Tick
  (if (Variables|Default|GetPlayerAndCameraMove)
    ;[1 1 1] Move Camera Along the Spline
    (if (Variables|Default|GetMoveCamera)
      (Transformation|SetActorLocation (Spline|GetLocationatDistanceAlongSpline (Variables|/Game/Assets/Blueprints/Spline_BP.Spline_BP_C|GetSpline (Variables|Default|GetSplineBP)) (Variables|Default|GetSplineDistance) "World") false false)
      (Variables|Default|SetSplineDistance (+ (Variables|Default|GetSplineDistance) (* (Utilities|Time|GetWorldDeltaSeconds) (Variables|Default|GetCameraSpeed)))))
    ;[1 1 1] Constantly moves the player downwards
    (Transformation|AddLocalOffset (Variables|Default|GetPlayer) (Utilities|FakeGravity) false false)
    ;[1 1 1] Player speed/movement
    (Variables|Default|SetVelocity (+ (Variables|Default|GetVelocity) (* (Utilities|PlayerVelocity) (Utilities|Time|GetWorldDeltaSeconds))))
    ;[1 1 1] Adds friction
    (bind _output_get (Variables|Default|SetVelocity (- (Variables|Default|GetVelocity) (* (* (Variables|Default|GetVelocity) (Variables|Default|GetPlayerFriction)) (Utilities|Time|GetWorldDeltaSeconds)))))
    ;[1 1 1] Moves the player
    (Transformation|AddLocalOffset (Variables|Default|GetPlayer) (* _output_get (Utilities|Time|GetWorldDeltaSeconds)) false false)
    ;[1 1 1] Rotates the player
    (Transformation|SetRelativeRotation (Variables|Default|GetSubmarine_mesh) (Math|Rotator|MakeRotator (+ (* (.z (Variables|Default|GetVelocity)) -0.05) (* (.y (Variables|Default|GetVelocity)) -0.01)) 0.0 0.0) false false)
    (if (or (!= (Variables|Default|GetInputHorizontal) 0.0) (!= (Variables|Default|GetInputVertical) 0.0))
      (Utilities|FlowControl|DoOnce true :!label _label
        (:Completed
          (Audio|Components|Audio|SetVolumeMultiplier _submarinemovement 0.45 :!class /Script/Engine.AudioComponent)))
      (else
        (Utilities|FlowControl|Sequence
          (:then_0
            (goto _label Reset))
          (:then_1
            (Audio|Components|Audio|SetVolumeMultiplier _submarinemovement 0.15 :!class /Script/Engine.AudioComponent)))))))

(event EventBeginPlay
  ;[1 1 1] Lock and show mouse cursor
  (Input|SetInputModeGameandUI (Game|GetPlayerController 0) 0 "LockAlways" false)
  (Variables|/Script/Engine.PlayerController|SetbShowMouseCursor (Game|GetPlayerController 0) true)
  (bind _assubmarine_con (Utilities|Casting|CastToSubmarine_Con (Game|GetPlayerController 0)))
  (Variables|Default|SetSubmarineCon _assubmarine_con)
  (if (Variables|Default|GetPlayerDeathAtStart)
    ;[1 1 1] If player death at start is true, kill player at start(For the menu)
    (Components|Activation|SetActive (Variables|Default|GetSubmarineMovement) false false)
    (Components|DestroyComponent (Variables|Default|GetPlayer))
    (Variables|Default|SetPlayerAndCameraMove false)
    (Default|MenuScreen (Variables|Default|GetSubmarineCon))))

(event Collision|EventActorBeginOverlap
  (params (OtherActor :type Actor%20Object%20Reference))
  ;[0.735 0.08452 0.08452] If the player collides with anything, it goes through the collision list of what will happen
  (CallFunction|Collision OtherActor))

(event Input|ActionEvents|InputActionStopCamera
  (params (Key :type Key%20Structure :default "AnyKey"))
  ;[0.735 0.08452 0.08452] Debuging Stuff
  (:Pressed
    (Variables|Default|SetCameraSpeed 0.0)
    (Development|PrintString "Stopping Camera")))

(event Input|ActionEvents|InputActionStartCamera
  (params (Key :type Key%20Structure :default "AnyKey"))
  ;[0.735 0.08452 0.08452] Debuging Stuff
  (:Pressed
    (Variables|Default|SetCameraSpeed 3.5e+02)
    (Development|PrintString "Camera Normal Speed")))

(event Input|ActionEvents|InputActionSpeedUpCamera
  (params (Key :type Key%20Structure :default "AnyKey"))
  ;[0.735 0.08452 0.08452] Debuging Stuff
  (:Pressed
    (Variables|Default|SetCameraSpeed (+ (Variables|Default|GetCameraSpeed) 1e+02))
    (Development|PrintString "Adding Camera Speed")))

(event Input|ActionEvents|InputActionPlayerInvisible
  (params (Key :type Key%20Structure :default "AnyKey"))
  ;[0.735 0.08452 0.08452] Debuging Stuff
  (:Pressed
    (Variables|Default|SetDebugCollision true)
    (Development|PrintString "Player Can't take damage")))

(event Input|ActionEvents|InputActionPlayerUnInvisible
  (params (Key :type Key%20Structure :default "AnyKey"))
  ;[0.735 0.08452 0.08452] Debuging Stuff
  (:Pressed
    (Variables|Default|SetDebugCollision false)
    (Development|PrintString "Player can take damage")))

(event Input|ActionEvents|InputActionFire
  (params (Key :type Key%20Structure :default "AnyKey"))
  (bind _submarinecon (Variables|Default|GetSubmarineCon))
  ;[0.735 0.08452 0.08452] Shoot a projectile
  (:Pressed
    (if (Variables|Default|GetPlayerAndCameraMove)
      (if (== (Variables|/Game/Assets/Blueprints/Gm_Con_HUD/Submarine_Con.Submarine_Con_C|GetCurrentProjectileDelay (Variables|Default|GetSubmarineCon)) 0.0)
        ;[1 1 1] Spawns a projectile at the submarine going in the direction of the aim
        (Utilities|FlowControl|DoOnce false :!label _label
          (:Completed
            (Audio|PlaySoundatLocation "/Game/Assets/Sounds/ProjectileEject.ProjectileEject" (Transformation|GetWorldLocation (Variables|Default|GetPlayer)))
            (Game|SpawnActorfromClass "/Game/Assets/Blueprints/Projectile_BP.Projectile_BP_C" (Math|Transform|MakeTransform (Transformation|GetWorldLocation (Variables|Default|GetAim self)) (Variables|/Game/Assets/Blueprints/Gm_Con_HUD/Submarine_Con.Submarine_Con_C|GetAimRotation (Variables|Default|GetSubmarineCon)) "1.000000,1,1") "AlwaysSpawn" 0 0)
            ;[1 1 1] Delay until you can shoot again
            (Variables|/Game/Assets/Blueprints/Gm_Con_HUD/Submarine_Con.Submarine_Con_C|SetCurrentProjectileDelay _submarinecon (Variables|/Game/Assets/Blueprints/Gm_Con_HUD/Submarine_Con.Submarine_Con_C|GetMaxProjectileDelay _submarinecon))
            (goto _label Reset)))))))

(event Input|AxisEvents|InputAxisHorizontalMove
  (params (AxisValue :type Float%20%28single-precision%29))
  ;[0.735 0.08452 0.08452] Axis movement, perrdy gud
  (Variables|Default|SetInputHorizontal AxisValue))

(event Input|AxisEvents|InputAxisLeftStickHorizontal
  (params (AxisValue :type Float%20%28single-precision%29))
  ;[0.735 0.08452 0.08452] Controller Input
)

(event Input|AxisEvents|InputAxisVerticalMove
  (params (AxisValue :type Float%20%28single-precision%29))
  ;[0.735 0.08452 0.08452] Axis movement, perrdy gud
  (Variables|Default|SetInputVertical AxisValue))

(event Input|AxisEvents|InputAxisLeftStickVertical
  (params (AxisValue :type Float%20%28single-precision%29))
  ;[0.735 0.08452 0.08452] Controller Input
)

(event Input|AxisEvents|InputAxisRightStickVertical
  (params (AxisValue :type Float%20%28single-precision%29))
  ;[0.735 0.08452 0.08452] Controller Input
)

(event Input|AxisEvents|InputAxisRightStickHorizontal
  (params (AxisValue :type Float%20%28single-precision%29))
  ;[0.735 0.08452 0.08452] Controller Input
)

(fn ConstructionScript)

(fn Collision
  (params (Other%20Actor :type Actor%20Object%20Reference))
  (Variables|Default|SetOtherActor Other%20Actor)
  (Utilities|FlowControl|Sequence
    (:then_0
      ;[1 1 1] If the other Actor is a Tentacle, make the Tentacle disappear for a while
      (if (Actor|ActorHasTag (Variables|Default|GetOtherActor) "Tentacle")
        (bind _assquid_arm_bp (Utilities|Casting|CastToSquidArm_BP (Variables|Default|GetOtherActor)))
        (Default|Impact _assquid_arm_bp)
        (else
          ;[1 1 1] If the other Actor is a Rock, destroy the rock
          (if (Actor|ActorHasTag (Variables|Default|GetOtherActor) "Rock")
            (bind _asdestructible_rock_bp (Utilities|Casting|CastToDestructibleRock_BP (Variables|Default|GetOtherActor)))
            (Default|Destroy _asdestructible_rock_bp)
            (else
              ;[1 1 1] If the other Actor is a Falling Rock, destroy the Falling rock
              (if (Actor|ActorHasTag (Variables|Default|GetOtherActor) "FallingRock")
                (bind _asfalling_rock_bp (Utilities|Casting|CastToFallingRock_BP (Variables|Default|GetOtherActor)))
                (Default|Destroy _asfalling_rock_bp)
                (elif (Actor|ActorHasTag (Variables|Default|GetOtherActor) "FirstRock")
                  (bind _asfirst_destructible_rock_bp (Utilities|Casting|CastToFirstDestructibleRock_BP (Variables|Default|GetOtherActor)))
                  (Default|Destroy _asfirst_destructible_rock_bp)
                  (elif (Actor|ActorHasTag (Variables|Default|GetOtherActor) "Mine")
                    (bind _asexplodable_mine_bp (Utilities|Casting|CastToExplodableMine_BP (Variables|Default|GetOtherActor)))
                    (Default|ExplodeMine _asexplodable_mine_bp)))))))))
    (:then_1
      ;[1 1 1] If the other Actor is a Pearl, add +1 to the total pearl collection
      (if (Actor|ActorHasTag (Variables|Default|GetOtherActor) "Pearl")
        (bind _ascollect_pearl_bp (Utilities|Casting|CastToCollectPearl_BP (Variables|Default|GetOtherActor)))
        (Default|CollectPearl _ascollect_pearl_bp)
        (else
          ;[1 1 1] If the other Actor is the BigPearl, win the game
          (if (Actor|ActorHasTag (Variables|Default|GetOtherActor) "GiantPearl")
            (Default|WinScreen (Variables|Default|GetSubmarineCon))
            (else
              ;[1 1 1] If the other Actor is Energy, add energy to the current amount of Energy
              (if (Actor|ActorHasTag (Variables|Default|GetOtherActor) "Energy")
                (bind _asenergy_pickup_bp (Utilities|Casting|CastToEnergyPickup_BP (Variables|Default|GetOtherActor)))
                (Default|CollectEnergy _asenergy_pickup_bp)
                (else
                  ;[1 1 1] If the other Actor is Energy, add energy to the current amount of Energy
                  (if (Actor|ActorHasTag (Variables|Default|GetOtherActor) "FullEnergy")
                    (bind _asfull_energy_pickup_bp (Utilities|Casting|CastToFullEnergyPickup_BP (Variables|Default|GetOtherActor)))
                    (Default|CollectFullEnergy _asfull_energy_pickup_bp)
                    (else
                      ;[1 1 1] Checks if the other actor is one the player should ignore
                      (if (not (Actor|ActorHasTag (Variables|Default|GetOtherActor) "Tech"))
                        (if (not (Actor|ActorHasTag (Variables|Default|GetOtherActor) "Anemone"))
                          ;[1 1 1] If the other actor is not in the ignore list, then it damages the player
                          (CallFunction|PlayerDamage))))))))))))))

(fn PlayerDamage
  (bind _submarinecon (Variables|Default|GetSubmarineCon))
  ;[1 1 1] Is the player Invincible/in debugging mode?
  (if (not (Variables|Default|GetDebugCollision))
    (if (not (Variables|Default|GetPlayerInvincible))
      ;[1 1 1] Lower Current Energy with choosen amount
      (Variables|/Game/Assets/Blueprints/Gm_Con_HUD/Submarine_Con.Submarine_Con_C|SetCurrentEnergy _submarinecon (- (Variables|/Game/Assets/Blueprints/Gm_Con_HUD/Submarine_Con.Submarine_Con_C|GetCurrentEnergy _submarinecon) (Variables|Default|GetEnergyLoss)))
      ;[1 1 1] Shake Screen
      (CallFunction|CameraShake "/Game/Assets/Blueprints/CrashShake_BP.CrashShake_BP_C")
      (Audio|PlaySoundatLocation "/Game/Assets/Sounds/BubbleExplosion.BubbleExplosion" (Transformation|GetWorldLocation (Variables|Default|GetPlayer)))
      ;[1 1 1] Make Player Invincible for a amount of time
      (CallFunction|Invincibility))))

(fn PlayerDeath
  ;[1 1 1] Spawns explosion particles at the player and stops the bubble particles
  (Effects|SpawnEmitteratLocation "/Game/Assets/Particles/BubbleExplosionv2.BubbleExplosionv2" (Transformation|GetWorldLocation (Variables|Default|GetSubmarine_mesh)))
  (Components|Activation|SetActive (Variables|Default|GetBubbles) false false)
  ;[1 1 1] Stops the player from being able to move/use the flashlight or shoot missiles
  (Variables|Default|SetPlayerAndCameraMove false)
  (Variables|/Game/Assets/Blueprints/Gm_Con_HUD/Submarine_Con.Submarine_Con_C|SetbRotateFlashligt? (Variables|Default|GetSubmarineCon) false)
  ;[1 1 1] Deactivates the flashlight and starts the crash screen
  (Rendering|Components|Light|SetIntensity (Variables|Default|GetSpotLight) 0.0)
  (Default|CrashScreen (Variables|Default|GetSubmarineCon))
  ;[1 1 1] Shake screen
  (CallFunction|CameraShake "/Game/Assets/Blueprints/CrashShake_BP.CrashShake_BP_C"))