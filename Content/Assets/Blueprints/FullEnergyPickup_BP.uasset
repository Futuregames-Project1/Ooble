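; Energy pearl pickup that fully restores the submarine's energy when collected.
; CollectFullEnergy sets CurrentEnergy to MaxEnergy on the Submarine_Con player controller, spawns a flash and sound, then destroys the actor.
; BeginPlay records start and offset end points for an up-and-down bob, but the timeline that lerps between them is never triggered.
; The +25 energy note on the collect event does not match its full refill.
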(event Custom|CollectFullEnergy
  (bind _returnvalue (Transformation|GetActorLocation))
  ;[1 1 1] Adds +25 to Current Energy and destroys the pickup
  (bind _assubmarine_con (Utilities|Casting|CastToSubmarine_Con (Game|GetPlayerController 0)))
  (Variables|/Game/Assets/Blueprints/Gm_Con_HUD/Submarine_Con.Submarine_Con_C|SetCurrentEnergy _assubmarine_con (Variables|/Game/Assets/Blueprints/Gm_Con_HUD/Submarine_Con.Submarine_Con_C|GetMaxEnergy _assubmarine_con))
  (Effects|SpawnEmitteratLocation "/Game/Assets/Particles/PickupFlash_Par.PickupFlash_Par" _returnvalue)
  (Audio|SpawnSoundatLocation "/Game/Assets/Sounds/PickUpEnergy.PickUpEnergy" _returnvalue)
  (Actor|DestroyActor))

(event EventBeginPlay
  ;[1 1 1] Setting the start and end point for the pearl fluctuating movement
  (Variables|Default|SetEnergyInitialPoint (Transformation|GetWorldLocation (Variables|Default|GetSphere)))
  (Transformation|AddWorldOffset (Variables|Default|GetDummyEndPoint) (.Location (Math|Transform|BreakTransform (Variables|Default|GetEnergyFluctuationEndPoint))) false false)
  (Variables|Default|SetEnergyWorldPoint (Transformation|GetWorldLocation (Variables|Default|GetDummyEndPoint))))

(fn ConstructionScript)