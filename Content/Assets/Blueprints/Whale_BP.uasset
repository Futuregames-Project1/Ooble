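; Whale actor that moves its Scene component each tick, driven by a spline.
; Tick samples Spline1's local-space location at SplineDistance, then advances that distance by WhaleSpeed scaled by world delta seconds.
; The sampled location is applied as an additive local offset rather than an absolute position, so movement accumulates each frame.
; The graph has no looping or reset of the distance, and the construction script is empty.
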(event EventTick
  (params (DeltaSeconds :type Float%20%28single-precision%29))
  (Transformation|AddLocalOffset (Variables|Default|GetScene) (Spline|GetLocationatDistanceAlongSpline (Variables|Default|GetSpline1) (Variables|Default|GetSplineDistance) "Local") false false)
  (Variables|Default|SetSplineDistance (+ (Variables|Default|GetSplineDistance) (* (Utilities|Time|GetWorldDeltaSeconds) (Variables|Default|GetWhaleSpeed)))))

(fn ConstructionScript)