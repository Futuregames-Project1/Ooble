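; FallingRock_BP is a breakable rock actor that moves along negative world X and removes itself after a timed lifetime.
; Tick offsets the destructible mesh by FallingSpeed scaled with frame time, without sweeping.
; Its Destroy event shrinks the actor, applies damage to fracture the destructible mesh, plays a cracking sound, disables static mesh collision, then destroys the actor after a delay.
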(event Custom|Destroy
  (bind _fallingrock_dm (Variables|Default|GetFallingRock_DM))
  (bind _returnvalue (Transformation|GetWorldLocation _fallingrock_dm))
  (Transformation|SetActorScale3D (* (Transformation|GetActorScale3D self) 0.25))
  (Game|Damage|ApplyDamage _fallingrock_dm 1.0 _returnvalue _returnvalue 0.0)
  (Audio|PlaySoundatLocation "/Game/Assets/Sounds/RocksCrack.RocksCrack" _returnvalue)
  (Collision|SetCollisionEnabled (Variables|Default|GetStaticMesh) "NoCollision")
  (Utilities|FlowControl|Delay 1e+01)
  (Actor|DestroyActor))

(event EventBeginPlay
  (Utilities|FlowControl|Delay 15.0)
  (Actor|DestroyActor))

(event EventTick
  (params (DeltaSeconds :type Float%20%28single-precision%29))
  (Transformation|AddWorldOffset (Variables|Default|GetFallingRock_DM) (Math|Vector|MakeVector (* (* (Utilities|Time|GetWorldDeltaSeconds) (Variables|Default|GetFallingSpeed)) -1.0) 0.0 0.0) false false))

(fn ConstructionScript)