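; SquidArm_BP is a squid tentacle actor that shrinks when its Impact event fires and later destroys itself.
; The SquidArm timeline offsets the scale saved at BeginPlay, reducing Z more than X and Y.
; Delays chained from the timeline's Update pin, rather than Finished, reverse the timeline after a few seconds and destroy the actor later.
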(event Custom|Impact
  ;[1 1 1] Shrink Tentacle
  (bind _newtrack_0 (Timeline|SquidArm Play)
    (:Update
      (Transformation|SetActorScale3D (+ (Variables|Default|GetStartScale) (* (Math|Vector|MakeVector -0.1 -0.1 -0.3) _newtrack_0)))
      (Utilities|FlowControl|Sequence
        (:then_0
          (Utilities|FlowControl|Delay 3.1)
          (Timeline|SquidArm Reverse))
        (:then_1
          (Utilities|FlowControl|Delay 1e+01)
          (Actor|DestroyActor))))))

(event EventTick
  (params (DeltaSeconds :type Float%20%28single-precision%29)))

(event EventBeginPlay
  (Variables|Default|SetStartScale (Transformation|GetActorScale3D)))

(fn ConstructionScript)