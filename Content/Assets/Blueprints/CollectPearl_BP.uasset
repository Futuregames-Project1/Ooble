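; Collectible pearl that adds one to the collected pearl count on the Submarine_Con player controller when its CollectPearl event runs.
; Collection also spawns a bubble explosion effect and pickup sound, then destroys the actor.
; BeginPlay caches start and end points, using an offset DummyEndPoint, for a timeline-lerped up-and-down bob.
; That timeline is never triggered in this graph, so the bobbing movement does not run.
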(event Custom|CollectPearl
  (bind _self self)
  (bind _returnvalue (Transformation|GetActorLocation _self))
  ;[1 1 1] Adds +1 to CollectedPearlAmount, spawns a particle effect and destroys the pearl
  (bind _assubmarine_con (Utilities|Casting|CastToSubmarine_Con (Game|GetPlayerController 0)))
  (Variables|/Game/Assets/Blueprints/Gm_Con_HUD/Submarine_Con.Submarine_Con_C|SetCollectedPearlAmount _assubmarine_con (+ (Variables|/Game/Assets/Blueprints/Gm_Con_HUD/Submarine_Con.Submarine_Con_C|GetCollectedPearlAmount _assubmarine_con) 1))
  (Effects|SpawnEmitteratLocation "/Game/Assets/Particles/BubbleExplosionv2.BubbleExplosionv2" _returnvalue)
  (Audio|SpawnSoundatLocation "/Game/Assets/Sounds/PickUpPearl.PickUpPearl" _returnvalue)
  (Actor|DestroyActor))

(event EventBeginPlay
  ;[1 1 1] Setting the start and end point for the pearl fluctuating movement
  (Variables|Default|SetPearlInitialPoint (Transformation|GetWorldLocation (Variables|Default|GetSphere)))
  (Transformation|AddWorldOffset (Variables|Default|GetDummyEndPoint) (.Location (Math|Transform|BreakTransform (Variables|Default|GetPearlFluctuationEndPoint))) false false)
  (Variables|Default|SetPearlWorldPoint (Transformation|GetWorldLocation (Variables|Default|GetDummyEndPoint))))

(fn ConstructionScript)