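; Projectile_BP is a missile projectile that damages obstacles on overlap in an underwater submarine game.
; Actor tags route each hit to a cast that calls Impact on squid arms or Destroy on the rock variants.
; Any overlap except pearl and energy pickups also runs DeactivateProjectile, which shakes the submarine camera, spawns a bubble explosion with sound, deactivates components and hides the missile.
; The actor is destroyed two seconds later.
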(event Collision|EventActorBeginOverlap
  (params (OtherActor :type Actor%20Object%20Reference))
  (Variables|Default|SetOtherActor OtherActor)
  (Utilities|FlowControl|Sequence
    (:then_0
      (if (Actor|ActorHasTag (Variables|Default|GetOtherActor) "Tentacle")
        (bind _assquid_arm_bp (Utilities|Casting|CastToSquidArm_BP (Variables|Default|GetOtherActor)))
        (Default|Impact _assquid_arm_bp)
        (elif (Actor|ActorHasTag (Variables|Default|GetOtherActor) "Rock")
          (bind _asdestructible_rock_bp (Utilities|Casting|CastToDestructibleRock_BP (Variables|Default|GetOtherActor)))
          (Default|Destroy _asdestructible_rock_bp)
          (elif (Actor|ActorHasTag (Variables|Default|GetOtherActor) "FallingRock")
            (bind _asfalling_rock_bp (Utilities|Casting|CastToFallingRock_BP (Variables|Default|GetOtherActor)))
            (Default|Destroy _asfalling_rock_bp)
            (elif (Actor|ActorHasTag (Variables|Default|GetOtherActor) "FirstRock")
              (bind _asfirst_destructible_rock_bp (Utilities|Casting|CastToFirstDestructibleRock_BP (Variables|Default|GetOtherActor)))
              (Default|Destroy _asfirst_destructible_rock_bp))))))
    (:then_1
      (if (not (Actor|ActorHasTag (Variables|Default|GetOtherActor) "Pearl"))
        (if (not (Actor|ActorHasTag (Variables|Default|GetOtherActor) "Energy"))
          (if (not (Actor|ActorHasTag (Variables|Default|GetOtherActor) "FullEnergy"))
            (CallFunction|DeactivateProjectile)
            (Utilities|FlowControl|Delay 2.0)
            (Actor|DestroyActor)))))))

(fn ConstructionScript)

(fn DeactivateProjectile
  (bind _defaultsceneroot (Variables|Default|GetDefaultSceneRoot))
  (bind _returnvalue (Transformation|GetWorldLocation _defaultsceneroot))
  (bind _assubmarine_bp (Utilities|Casting|CastToSubmarine_BP (Game|Player|GetPlayerPawn 0)))
  (Default|CameraShake _assubmarine_bp "/Game/Assets/Blueprints/MissileShake_BP.MissileShake_BP_C")
  (Effects|SpawnEmitteratLocation "/Game/Assets/Particles/BubbleExplosionv2.BubbleExplosionv2" _returnvalue)
  (Audio|PlaySoundatLocation "/Game/Assets/Sounds/BubbleExplosion.BubbleExplosion" _returnvalue)
  (Components|Activation|SetActive (Variables|Default|GetProjectileMovement) false false)
  (Rendering|SetVisibility (Variables|Default|GetMissile) false false))