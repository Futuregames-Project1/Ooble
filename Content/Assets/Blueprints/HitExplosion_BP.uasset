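; HitExplosion_BP is a self-destroying actor that plays a grow-then-shrink hit explosion effect on its ImplosionRadiusSphere.
; On BeginPlay, one timeline lerps the sphere from OriginalScale to NewScale, and a second lerps it back.
; Delays chained from each timeline's Update pin, rather than Finished, trigger the next stage.
; The sphere then switches to a see-through material and the actor destroys itself shortly after.
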(event EventBeginPlay
  (bind _originalscale (Variables|Default|GetOriginalScale))
  (bind _implosionradiussphere (Variables|Default|GetImplosionRadiusSphere))
  (Transformation|SetRelativeScale3D _implosionradiussphere _originalscale)
  (bind _scaletrack (Timeline|Timeline_0 PlayFromStart)
    (:Update
      (Transformation|SetRelativeScale3D _implosionradiussphere (Math|Vector|Lerp(Vector) _originalscale (Variables|Default|GetNewScale) _scaletrack))
      (Utilities|FlowControl|Delay 0.5)
      (bind _scaletrack_2 (Timeline|Timeline_1 PlayFromStart)
        (:Update
          (Transformation|SetRelativeScale3D (Variables|Default|GetImplosionRadiusSphere) (Math|Vector|Lerp(Vector) (Variables|Default|GetNewScale) (Variables|Default|GetOriginalScale) _scaletrack_2))
          (Utilities|FlowControl|Delay 0.5)
          (Rendering|Material|SetMaterial (Variables|Default|GetImplosionRadiusSphere) 0 "/Game/Assets/Materials/SeeThroughWindowTransparent_Mat.SeeThroughWindowTransparent_Mat")
          (Utilities|FlowControl|Delay 2.0)
          (Actor|DestroyActor))))))

(event Collision|EventActorBeginOverlap
  (params (OtherActor :type Actor%20Object%20Reference)))

(event EventTick
  (params (DeltaSeconds :type Float%20%28single-precision%29)))

(fn ConstructionScript)