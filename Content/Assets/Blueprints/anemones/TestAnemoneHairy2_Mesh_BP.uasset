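; Hairy anemone test Blueprint that lights up the first time an actor overlaps it.
; A DoOnce gate starts timelines that animate the point light's attenuation radius and the mesh's EmissiveBoostTendril material parameter.
; Each radius update also restarts an intensity timeline, which sets the light to a fixed intensity rather than a curve value.
; The gate is never reset, so the glow triggers only once.
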(event EventBeginPlay)

(event Collision|EventActorBeginOverlap
  (params (OtherActor :type Actor%20Object%20Reference))
  (Utilities|FlowControl|DoOnce false
    (:Completed
      (Utilities|FlowControl|Sequence
        (:then_0
          (bind _newtrack_0 (Timeline|Attenuation%20Radius PlayFromStart)
            (:Update
              (Rendering|Lighting|SetAttenuationRadius (Variables|Default|GetPointLight) _newtrack_0)
              (Timeline|PointLightIntensity PlayFromStart
                (:Update
                  (Rendering|Components|Light|SetIntensity (Variables|Default|GetPointLight) 3e+02))))))
        (:then_1
          (bind _newtrack_0_2 (Timeline|EmissiveBoost PlayFromStart)
            (:Update
              (Rendering|Material|SetScalarParameterValueonMaterials (Variables|Default|GetStaticMesh) "EmissiveBoostTendril" _newtrack_0_2))))))))

(event EventTick
  (params (DeltaSeconds :type Float%20%28single-precision%29)))

(fn ConstructionScript)