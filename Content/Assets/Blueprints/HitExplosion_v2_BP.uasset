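; HitExplosion_v2_BP is a self-destroying explosion effect actor, driven entirely from BeginPlay by timelines and delays.
; ImplosionRadiusSphere grows, animates opacity, shrinks, then switches to a transparent material before the actor is destroyed.
; In parallel, LightningSphere scales up, animates its opacity and spawns the BubbleExplosionv1 emitter.
; Each stage chains from the previous timeline's Update pin rather than Finished, so downstream timelines and delays are retriggered every update.
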(event EventBeginPlay
  (bind _lightningsphere (Variables|Default|GetLightningSphere))
  (bind _implosionradiussphere (Variables|Default|GetImplosionRadiusSphere))
  (bind _originalscale (Variables|Default|GetOriginalScale))
  (Transformation|SetRelativeScale3D _implosionradiussphere _originalscale)
  (bind _scaletrack (Timeline|RefractSphereIncrease PlayFromStart)
    (:Update
      (Transformation|SetRelativeScale3D _implosionradiussphere (Math|Vector|Lerp(Vector) _originalscale (Variables|Default|GetNewScale) _scaletrack))
      (Utilities|FlowControl|Sequence
        (:then_0
          (Utilities|FlowControl|Delay 1.0)
          (bind _lightsphereexpand (Timeline|Timeline_0 PlayFromStart)
            (:Update
              (Rendering|Material|SetScalarParameterValueonMaterials (Variables|Default|GetImplosionRadiusSphere) "Opacity" _lightsphereexpand)
              (Utilities|FlowControl|Delay 2.0)
              (bind _scaletrack_2 (Timeline|RefractionDecrease PlayFromStart)
                (:Update
                  (Transformation|SetRelativeScale3D (Variables|Default|GetImplosionRadiusSphere) (Math|Vector|Lerp(Vector) (Variables|Default|GetNewScale) (Variables|Default|GetOriginalScale) _scaletrack_2))
                  (Utilities|FlowControl|Delay 0.5)
                  (Rendering|Material|SetMaterial (Variables|Default|GetImplosionRadiusSphere) 0 "/Game/Assets/Materials/SeeThroughWindowTransparent_Mat.SeeThroughWindowTransparent_Mat")
                  (Utilities|FlowControl|Delay 2.0)
                  (Actor|DestroyActor))))))
        (:then_1
          (bind _scaletrack_3 (Timeline|LightningIncrease PlayFromStart)
            (:Update
              (Transformation|SetRelativeScale3D _lightningsphere (Math|Vector|Lerp(Vector) "1.000000,1.000000,1.000000" "4.000000,4.000000,4.000000" _scaletrack_3))
              (bind _lightsphereexpand_2 (Timeline|SphereOpacity PlayFromStart)
                (:Update
                  (Rendering|Material|SetScalarParameterValueonMaterials _lightningsphere "OpacityMult" _lightsphereexpand_2)
                  (Utilities|FlowControl|Delay 0.7)
                  (Effects|SpawnEmitteratLocation "/Game/Assets/Particles/BubbleExplosionv1.BubbleExplosionv1" (Transformation|GetWorldLocation _lightningsphere)))))))))))

(event Collision|EventActorBeginOverlap
  (params (OtherActor :type Actor%20Object%20Reference)))

(event EventTick
  (params (DeltaSeconds :type Float%20%28single-precision%29)))

(fn ConstructionScript)